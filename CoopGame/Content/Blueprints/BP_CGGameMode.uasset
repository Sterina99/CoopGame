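; Game mode Blueprint that spawns enemy bots and awards score for kills.
; SpawnNewBot runs an EQS spawn-location query, then debug-draws each returned location and spawns either an advanced AI or, more often, a tracker bot there.
; On BeginPlay it binds to the actor-killed event, adding points to the killer's player state and printing the score when the victim is a non-player pawn.
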(event Custom|OnQueryFinishedEvent_Event_0
  (params (QueryInstance :type Env%20Query%20Instance%20Blueprint%20Wrapper%20Object%20Reference) (QueryStatus :type EEnvQueryStatus%20Enum :default "Processing"))
  (switch Utilities|FlowControl|Switch|SwitchonEEnvQueryStatus QueryStatus
    (:Success
      (bind _resultlocations (AI|EQS|GetQueryResultsasLocations QueryInstance))
      (for _array_element _resultlocations
        (Rendering|Debug|DrawDebugSphere _array_element 1e+02 12 "(R=0.974842,G=1.000000,B=0.016521,A=1.000000)" 2.0 2.0)
        (Game|SpawnActorfromClass (select (<= (Math|Random|RandomFloatinRange 0.0 1e+02) 33.0) "/Game/AdvancedAI/BP_AdvancedAI.BP_AdvancedAI_C" "/Game/TrackerBot/BP_CGTrackerBot.BP_CGTrackerBot_C") (Math|Transform|MakeTransform _array_element) "AdjustIfPossibleButAlwaysSpawn" 0 0)))))

(event Custom|OnActorKilled_Event_0
  (params (VictimActor :type Actor%20Object%20Reference) (KillerActor :type Actor%20Object%20Reference) (KillerController :type Controller%20Object%20Reference))
  (bind _aspawn (Utilities|Casting|CastToPawn VictimActor))
  (if (not (Pawn|IsPlayerControlled _aspawn))
    (bind _ascgplayer_state (Utilities|Casting|CastToCGPlayerState (Variables|/Script/Engine.Pawn|GetPlayerState (Pawn|GetControlledPawn KillerController))))
    (Class|CGPlayerState|AddScore _ascgplayer_state 2e+01)
    (Development|PrintString (Utilities|String|ToString(Float) (Variables|/Script/Engine.PlayerState|GetScore _ascgplayer_state)) true true "(R=0.000000,G=1.000000,B=0.462500,A=1.000000)")))

(event EventBeginPlay
  (EventDispatchers|AssignOnActorKilled (delegate Custom|OnActorKilled_Event_0)))

(event EventTick
  (params (DeltaSeconds :type Float%20%28single-precision%29)))

(event EventSpawnNewBot
  (bind _returnvalue (AI|EQS|RunEQSQuery "/Game/Blueprints/EQS_FindSpawnLocation.EQS_FindSpawnLocation" self "RandomBest25Pct"))
  (EventDispatchers|AssignOnQueryFinishedEvent _returnvalue (delegate Custom|OnQueryFinishedEvent_Event_0)))

(fn ConstructionScript)