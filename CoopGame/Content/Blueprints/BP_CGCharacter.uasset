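; BP_CGCharacter is a character Blueprint with a health HUD and a basic shoot input.
; On BeginPlay, only the locally controlled instance creates a WBP_HealthIndicator widget and adds it to the viewport.
; Left mouse press pulses the Shoot flag true for a brief delay before clearing it.
; Tick prints an on-screen debug string for the locally controlled character.
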(event EventBeginPlay
  (if (Pawn|IsLocallyControlled)
    (bind _returnvalue (UserInterface|CreateWidget "/Game/UI/WBP_HealthIndicator.WBP_HealthIndicator_C"))
    (UserInterface|Viewport|AddtoViewport _returnvalue 0)))

(event Collision|EventActorBeginOverlap
  (params (OtherActor :type Actor%20Object%20Reference)))

(event EventTick
  (params (DeltaSeconds :type Float%20%28single-precision%29))
  (if (Pawn|IsLocallyControlled)
    (Development|PrintString "Hello" true false "(R=0.813331,G=1.000000,B=0.000000,A=1.000000)" 0.0)))

(event Input|MouseEvents|LeftMouseButton
  (params (Key :type Key%20Structure :default "None"))
  (:Pressed
    (Variables|Default|SetShoot true)
    (Utilities|FlowControl|Delay 0.1)
    (Variables|Default|SetShoot false)))

(fn ConstructionScript)