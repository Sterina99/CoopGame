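; Super-speed power-up that temporarily doubles the walk speed of the player who activates it.
; OnActivated stores that player and sets its CharacterMovementComponent's MaxWalkSpeed to twice the current GetMaxSpeed value.
; OnExpired halves the then-current max speed, rather than restoring a saved value, if the player is still valid, then calls the parent's expiry logic.
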(event EventBeginPlay)

(event Collision|EventActorBeginOverlap
  (params (OtherActor :type Actor%20Object%20Reference)))

(event EventTick
  (params (DeltaSeconds :type Float%20%28single-precision%29)))

(event EventOnExpired
  (bind _activate_for_player (Variables|Default|GetActivate%20For%20Player))
  (bind _returnvalue (Actor|GetComponentbyClass _activate_for_player "/Script/Engine.CharacterMovementComponent"))
  (Utilities|IsValid _activate_for_player
    (:Is%20Valid
      (Variables|/Script/Engine.CharacterMovementComponent|SetMaxWalkSpeed _returnvalue (/ (Class|MovementComponent|GetMaxSpeed _returnvalue) 2.0)))
    (:Is%20Not%20Valid
      _))
  (|CallParentFunction))

(event EventOnActivated
  (params (ActivateFor :type Actor%20Object%20Reference))
  (bind _returnvalue (Actor|GetComponentbyClass ActivateFor "/Script/Engine.CharacterMovementComponent"))
  (Variables|Default|SetActivate%20For%20Player ActivateFor)
  (Variables|/Script/Engine.CharacterMovementComponent|SetMaxWalkSpeed _returnvalue (* (Class|MovementComponent|GetMaxSpeed _returnvalue) 2.0)))

(fn ConstructionScript)